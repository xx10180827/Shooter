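; Shooter is a player-controlled character with axis-driven movement, look and a held-fire automatic hitscan weapon.
; Pressing fire plays a montage, attaches a muzzle flash, shoots immediately and repeats on a looping timer until release clears all three.
; Each shot line-traces from the camera along control rotation, leaves persistent debug lines and applies fixed damage to any Boot_Shooter_BP hit.
; Jump is movement input along the control up vector.
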(event EventBeginPlay)

(event Collision|EventActorBeginOverlap
  (params (OtherActor :type Actor%20Object%20Reference)))

(event EventTick
  (params (DeltaSeconds :type Float%20%28single-precision%29)))

(event Input|ActionEvents|InputActionfire
  (params (Key :type Key%20Structure :default "AnyKey"))
  (:Pressed
    (CallFunction|StartFire))
  (:Released
    (CallFunction|EndFire)))

(event Input|AxisEvents|InputAxisMove_forward
  (params (AxisValue :type Float%20%28single-precision%29))
  (Pawn|Input|AddMovementInput (Math|Vector|GetForwardVector (Pawn|GetControlRotation :!class /Script/Engine.Pawn)) AxisValue false))

(event Input|AxisEvents|InputAxisJump
  (params (AxisValue :type Float%20%28single-precision%29))
  (Pawn|Input|AddMovementInput (Math|Vector|GetUpVector (Pawn|GetControlRotation :!class /Script/Engine.Pawn)) AxisValue false))

(event Input|AxisEvents|InputAxisMove_right
  (params (AxisValue :type Float%20%28single-precision%29))
  (Pawn|Input|AddMovementInput (Math|Vector|GetRightVector (Pawn|GetControlRotation :!class /Script/Engine.Pawn)) AxisValue false))

(event Input|AxisEvents|InputAxisturn_x
  (params (AxisValue :type Float%20%28single-precision%29))
  (Pawn|Input|AddControllerYawInput AxisValue))

(event Input|AxisEvents|InputAxisturn_y
  (params (AxisValue :type Float%20%28single-precision%29))
  (Pawn|Input|AddControllerPitchInput AxisValue))

(fn ConstructionScript)

(fn StartFire
  (Utilities|FlowControl|Sequence
    (:then_0
      (Animation|PlayAnimMontage "/Game/Blueprints/Shooter_fire_Montage.Shooter_fire_Montage" 1.0 "None")
      (bind _returnvalue (Effects|SpawnEmitterAttached "/Game/Assets/Effects/ParticleSystems/Weapons/AssaultRifle/Muzzle/P_AssaultRifle_MF.P_AssaultRifle_MF" (Variables|Default|GetMuzzle) "None"))
      (Variables|Default|SetFire_%20Effect _returnvalue))
    (:then_1
      (CallFunction|ShootOnce)
      (Utilities|Time|SetTimerbyFunctionName 0 "Shoot_once" 0.2 true))))

(fn EndFire
  (Utilities|FlowControl|Sequence
    (:then_0
      (Animation|StopAnimMontage "/Game/Blueprints/Shooter_fire_Montage.Shooter_fire_Montage")
      (Components|DestroyComponent (Variables|Default|GetFire_%20Effect)))
    (:then_1
      (Utilities|Time|ClearTimerbyFunctionName 0 "Shoot_Once"))))

(fn ShootOnce
  (bind _camera (Variables|Default|GetCamera))
  (bind _returnvalue (Transformation|GetWorldLocation _camera))
  (bind (_outhit _returnvalue_2) (Collision|LineTraceByChannel _returnvalue (+ (* (Math|Vector|Normalize (Math|Vector|GetForwardVector (Pawn|GetControlRotation :!class /Script/Engine.Pawn))) 1.5e+03) _returnvalue) "TraceTypeQuery1" false 0 "Persistent"))
  (if _returnvalue_2
    (bind _asboot_shooter_bp (Utilities|Casting|CastToBoot_Shooter_BP (.HitActor (Collision|BreakHitResult _outhit))))
    (Default|TakeDamage _asboot_shooter_bp 2e+01)))