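; Shooter AI character Blueprint that reacts to GAS health and death events, with debug prints for both.
; BeginPlay binds a health-change handler, which loops back through the same bind and prints the new health.
; Death start detaches the controller, replacing an unwired IsDead check in TakeDamage, which now only prints health; ClearDeath destroys the actor.
; The construction script makes the mesh block the Visibility channel.
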(event Custom|CustomEvent
  (params (OldHealth :type Float%20%28single-precision%29) (NewHealth :type Float%20%28single-precision%29))
  ;[0.15 0.15 0.15 0.5] 扣血机制
  (EventDispatchers|BindEventtoOnGASHealthChanged (delegate Custom|CustomEvent))
  (Development|PrintString (Utilities|String|ToString(Float) NewHealth)))

(event EventBeginPlay
  ;[0.15 0.15 0.15 0.5] 扣血机制
  (EventDispatchers|BindEventtoOnGASHealthChanged (delegate Custom|CustomEvent))
  (Development|PrintString (Utilities|String|ToString(Float) (stale Custom|CustomEvent NewHealth))))

(event Collision|EventActorBeginOverlap
  (params (OtherActor :type Actor%20Object%20Reference)))

(event EventOnGASDeathStarted
  ;[0.15 0.15 0.15 0.5] AI死亡
  (Class|Pawn|DetachfromControllerPendingDestroy)
  (Development|PrintString "OnDeathStart"))

(fn ConstructionScript
  (Collision|SetCollisionResponsetoChannel (Variables|Character|GetMesh) "ECC_Visibility" "ECR_Block"))

(fn TakeDamage
  (params (Damage :type Float%20%28double-precision%29))
  (Development|PrintString (Utilities|String|ToString(Float) (Class|ShooterCharacterBase|GetGASHealth))))

(fn IsDead
  (return (<= (Class|ShooterCharacterBase|GetGASHealth) 0.0)))

(fn ClearDeath
  (Actor|DestroyActor))